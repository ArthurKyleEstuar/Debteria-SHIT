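; Coffee cup projectile that applies a hit to what it overlaps and then detonates.
; Box overlaps call DidHit on any actor not tagged Wall, then Detonate runs in every case, walls included.
; When destroyed, it spawns a BaseEffect at its location.
; SetShadowPos only traces downward from the actor; the trace result never moves anything.
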(event `self.ReceiveTick`
  (params (DeltaSeconds :type "Float (single-precision)")))

(event `self.Box.OnComponentBeginOverlap`
  (params (OverlappedComponent :type "PrimitiveComponent Object Reference") (OtherActor :type "Actor Object Reference") (OtherComp :type "PrimitiveComponent Object Reference") (OtherBodyIndex :type Integer) (bFromSweep :type Boolean) (SweepResult :type "HitResult Structure (by ref)"))
  (if (not (`self.ActorHasTag` OtherActor "Wall"))
    (`/Game/Scripts/Blueprints/Projectile/ProjectileMacroLibrary.didHit` OtherActor OtherComp
      (:`true`
        _)))
  (`self.Detonate`))

(event `self.ReceiveDestroyed`
  (`|SpawnActorFromClass` "/Game/Scripts/Blueprints/Effects/BaseEffect.BaseEffect_C" (`KismetMathLibrary.MakeTransform` (`self.K2_GetActorLocation`)) "Undefined" "OverrideRootScale" null 0.13 null))

(fn `SetShadowPos`
  (bind _returnvalue (`self.K2_GetActorLocation`))
  (bind _outhit (`KismetSystemLibrary.LineTraceSingleForObjects` _returnvalue (`KismetMathLibrary.MakeVector` (.x _returnvalue) (.y _returnvalue) (- (.z _returnvalue) 1000.0)) (`|MakeArray` "ObjectTypeQuery2" "ObjectTypeQuery1" :!type "EObjectTypeQuery Enum"))))

(fn `UserConstructionScript`
  (`parent.UserConstructionScript`))