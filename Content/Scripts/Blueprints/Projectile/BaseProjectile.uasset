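; Base projectile class that damages tagged targets, notifies its owner of hits and applies knockback and optional knockdown.
; HitTarget damages one actor, while Detonate damages every valid overlap in its box; both check actor and component tags and send results through message calls.
; Effects go to all valid overlaps, then the projectile optionally destroys itself.
; Overlap, continuous and destruction-effect events are empty stubs, with spawn sound and lifespan set on BeginPlay.
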(event `self.ReceiveBeginPlay`
  (`self.SetLifeSpan` (`self.LifeSpan`))
  (`GameplayStatics.PlaySoundAtLocation` (`self.sfxToPlay`) (`self.K2_GetActorLocation`)))

(event `self.Box.OnComponentBeginOverlap`
  (params (OverlappedComponent :type "PrimitiveComponent Object Reference") (OtherActor :type "Actor Object Reference") (OtherComp :type "PrimitiveComponent Object Reference") (OtherBodyIndex :type Integer) (bFromSweep :type Boolean) (SweepResult :type "HitResult Structure (by ref)")))

(event `Continous`)

(event `Start Hit Cooldown`
  (set `self.isHitCooldown` true)
  (`KismetSystemLibrary.Delay` 0.2)
  (set `self.isHitCooldown` false))

(event `DestructionEffect`)

(event `self.ReceiveDestroyed`
  (`self.DestructionEffect`))

(fn `ApplyEffects`
  (params (Targets :type "Array of Actor Object Reference"))
  (for _array_element Targets
    (message `/Game/Scripts/Blueprints/System/I_Damageable.Knockback` _array_element (`self.knockForce`))
    (if (`self.willKD`)
      (message `/Game/Scripts/Blueprints/System/I_Damageable.KnockDown` _array_element (`self.KDTime`))))
  (return))

(fn `DestroyOnContact`
  (if (`self.willDestroyOnContact`)
    (`self.DestructionEffect`)
    (`self.K2_DestroyActor`)))

(fn `Detonate`
  (for _array_element (`PrimitiveComponent.GetOverlappingComponents` (`self.Box`))
    (bind _returnvalue (`ActorComponent.GetOwner` _array_element))
    (if (and (`ActorComponent.ComponentHasTag` _array_element (`self.targetHitBox`)) (`self.ActorHasTag` _returnvalue (`self.target`)))
      (message `/Game/Scripts/Blueprints/System/I_Damageable.Take Damage` _returnvalue (`self.Damage`) (`self.Damage Type`) (`self.CritProjectile`) (`self.LowestDamage`))
      (message `/Game/Scripts/Blueprints/System/I_Damageable.HitSuccess` (`self.projectileOwner`))))
  (`self.ApplyEffects` (`self.GetValidTargets`))
  (`self.DestroyOnContact`))

(fn `GetValidTargets`
  (returns (Targets :type "Array of Actor Object Reference"))
  (locals (validTargets :type "Array of Actor Object Reference"))
  (for _array_element (`PrimitiveComponent.GetOverlappingComponents` (`self.Box`))
    (bind _returnvalue (`ActorComponent.GetOwner` _array_element))
    (if (and (`ActorComponent.ComponentHasTag` _array_element (`self.targetHitBox`)) (`self.ActorHasTag` _returnvalue (`self.target`)))
      (`KismetArrayLibrary.Array_Add` (`local.validTargets`) _returnvalue)))
  (return (`local.validTargets`)))

(fn `HitTarget`
  (params (TargetActor :type "Actor Object Reference") (TargetComp :type "ActorComponent Object Reference"))
  (if (and (`self.ActorHasTag` TargetActor (`self.target`)) (`ActorComponent.ComponentHasTag` TargetComp (`self.targetHitBox`)))
    (message `/Game/Scripts/Blueprints/System/I_Damageable.Take Damage` TargetActor (`self.Damage`) (`self.Damage Type`) (`self.CritProjectile`) (`self.LowestDamage`))
    (message `/Game/Scripts/Blueprints/System/I_Damageable.HitSuccess` (`self.projectileOwner`))
    (`self.ApplyEffects` (`self.GetValidTargets`))
    (`self.DestroyOnContact`)))

(fn `IsValidTarget`
  (params (targetActor :type "Actor Object Reference") (targetComponent :type "ActorComponent Object Reference"))
  (returns (isValidTarget :type Boolean))
  (return (and (`self.ActorHasTag` targetActor (`self.target`)) (`ActorComponent.ComponentHasTag` targetComponent (`self.targetHitBox`)))))

(fn `UserConstructionScript`)