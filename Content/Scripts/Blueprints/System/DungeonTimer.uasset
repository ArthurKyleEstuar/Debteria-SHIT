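; Dungeon countdown timer that fails the quest when the dungeon time runs out.
; On begin play it adds a timer widget holding a reference to itself, plays a tutorial prompt and waits on a Delay of DungeonTime, while Tick separately decrements that value.
; Expiry shows a failure popup, then a failed-mission screen.
; Closing that screen revives a dead player, saves data and fails the quest through the game instance.
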(event `self.ReceiveBeginPlay`
  (bind _returnvalue (`|CreateWidget` "/Game/Scripts/Blueprints/UI/SystemUI/TimerUI.TimerUI_C" null self))
  (`UserWidget.AddToViewport` _returnvalue 0)
  (`KismetSystemLibrary.Delay` 0.2)
  (`/Game/Scripts/Blueprints/MyGameInstance.PlayTutorialPrompt` (`/Game/Scripts/Blueprints/System/GetUtilities.GetMyGameInstance`) "Timer")
  (`KismetSystemLibrary.Delay` (`self.DungeonTime`))
  (bind _returnvalue_2 (`|CreateWidget` "/Game/Scripts/Blueprints/UI/SpecialEffectsUI/TextNotifPopupUI.TextNotifPopupUI_C" null "QUEST FAILED"))
  (`UserWidget.AddToViewport` _returnvalue_2 0)
  (`KismetSystemLibrary.Delay` 2.0)
  (bind _returnvalue_3 (`|CreateWidget` "/Game/Scripts/Blueprints/UI/QuestsUI/FailedMissionUI.FailedMissionUI_C"))
  (`UserWidget.AddToViewport` _returnvalue_3 0)
  (add `/Game/Scripts/Blueprints/UI/QuestsUI/FailedMissionUI.UIClosed` _returnvalue_3 (delegate `TP`)))

(event `TP`
  (bind _asbase_character (`/Game/Scripts/Blueprints/System/GetUtilities.GetPlayerCharacter`))
  (if (`/Game/Scripts/Blueprints/Characters/Player/BaseCharacter.isDead` _asbase_character)
    (`/Game/Scripts/Blueprints/Characters/Player/BaseCharacter.Revive` _asbase_character))
  (`/Game/Scripts/Blueprints/Characters/Player/BaseCharacter.Save Data` _asbase_character)
  (`/Game/Scripts/Blueprints/MyGameInstance.FailQuestNoRevive` (`/Game/Scripts/Blueprints/System/GetUtilities.GetMyGameInstance`)))

(event `self.ReceiveTick`
  (params (DeltaSeconds :type "Float (single-precision)"))
  (set `self.DungeonTime` (`KismetMathLibrary.FClamp` (- (`self.DungeonTime`) DeltaSeconds) 0.0 500.0)))

(fn `UserConstructionScript`)