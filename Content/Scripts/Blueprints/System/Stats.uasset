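; Stats component holding an actor's HP, spell slots, stamina, money, combat attributes and movement speed, with functions to query and modify them.
; TakeDamage scales damage by a five-element weakness cycle, subtracts the passed bonus defense and spawns floating damage numbers at the owner's screen position.
; A separate luck-weighted roll out of 20 applies crits, and money changes show a gain/loss widget.
; Most stats convert to and from a save struct.
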(fn `AddSpellSlot`
  (params (addAmount :type "Float (double-precision)"))
  (set `self.SpellSlots` (`KismetMathLibrary.FClamp` (+ addAmount (`self.SpellSlots`)) 0.0 (`self.maxSpellSlots`))))

(fn `CheckDeath`
  (returns (isDead :type Boolean))
  (return (<= (`self.HP`) 0.5)))

(fn `CheckForCrit`
  (params (BonusLUK :type Integer) (damage :type "Float (double-precision)"))
  (returns (appliedDamage :type "Float (double-precision)") (wasCrit :type Boolean))
  (if (>= (`KismetMathLibrary.RandomIntegerInRange` (+ BonusLUK (`self.LUK`)) 20) 20)
    (return (* damage (`self.critModifier`)) true)
    (else
      (return damage false))))

(fn `CheckForExhaustion`
  (returns (isExhausted :type Boolean))
  (return (<= (`self.curStamina`) 0)))

(fn `DisplayDamage`
  (params (damageTaken :type "Float (double-precision)") (isCrit :type Boolean))
  (bind _returnvalue (`KismetStringLibrary.Conv_IntToString` (`KismetMathLibrary.FTrunc` damageTaken)))
  (bind _screenposition (`GameplayStatics.ProjectWorldToScreen` (`GameplayStatics.GetPlayerController` 0) (`Actor.K2_GetActorLocation` (`self.GetOwner`)) true))
  (if isCrit
    (bind _returnvalue_2 (`|CreateWidget` "/Game/Scripts/Blueprints/UI/MainHUD/DamageNumbers.DamageNumbers_C" null _screenposition (`KismetStringLibrary.Concat_StrStr` _returnvalue "!")))
    (`UserWidget.AddToViewport` _returnvalue_2 0)
    (else
      (bind _returnvalue_3 (`|CreateWidget` "/Game/Scripts/Blueprints/UI/MainHUD/DamageNumbers.DamageNumbers_C" null _screenposition _returnvalue))
      (`UserWidget.AddToViewport` _returnvalue_3 0))))

(fn `EvaluateElementalAffinity`
  (params (otherElementType :type "/Game/Scripts/Blueprints/System/ElementType Enum" :default "NewEnumerator0"))
  (returns (elementBonus :type "Float (double-precision)"))
  (switch `/Game/Scripts/Blueprints/System/ElementType` otherElementType
    (:`NewEnumerator0`
      (`self.CheckIsElement` "NewEnumerator1"
        (:`true`
          _)
        (:`false`
          (return 1.0))))
    (:`NewEnumerator1`
      (`self.CheckIsElement` "NewEnumerator2"
        (:`true`
          _)
        (:`false`
          (return 1.0))))
    (:`NewEnumerator2`
      (`self.CheckIsElement` "NewEnumerator3"
        (:`true`
          _)
        (:`false`
          (return 1.0))))
    (:`NewEnumerator3`
      (`self.CheckIsElement` "NewEnumerator4"
        (:`true`
          _)
        (:`false`
          (return 1.0))))
    (:`NewEnumerator4`
      (`self.CheckIsElement` "NewEnumerator0"
        (:`true`
          _)
        (:`false`
          (return 1.0)))))
  (return 1.2))

(fn `EvaluteCrit`
  (params (isCrit :type Boolean))
  (returns (critModifier :type "Float (double-precision)"))
  (if isCrit
    (return 2.0)
    (else
      (return 1.0))))

(fn `Get HP Percentile`
  (returns (PercentileHP :type "Float (double-precision)"))
  (return (/ (`self.HP`) (`self.maxHP`))))

(fn `Get HP Values`
  (returns (HP :type "Float (double-precision)") (maxHP :type "Float (double-precision)"))
  (return (`self.HP`) (`self.maxHP`)))

(fn `GetAllStats asStruct`
  (returns (SaveData :type "/Game/Scripts/Blueprints/System/Data/PlayerSaveData Structure"))
  (return (make `/Game/Scripts/Blueprints/System/Data/PlayerSaveData` (`self.maxHP`) (`self.HP`) (`self.ATK`) (`self.DEF`) (`self.Money`) (`self.maxSpellSlots`) (`self.SpellSlots`) (`self.LUK`) (`self.critModifier`) (`self.Name`) (`self.curStamina`) (`self.movementSpeed`))))

(fn `GetSpellSlot Values`
  (returns (SpellSlots :type "Float (double-precision)") (maxSpellSlots :type "Float (double-precision)"))
  (return (`self.SpellSlots`) (`self.maxSpellSlots`)))

(fn `GetSpellSlotPercentile`
  (returns (percentileSpellSlot :type "Float (double-precision)"))
  (return (/ (`self.SpellSlots`) (`self.maxSpellSlots`))))

(fn `RecoverMovmentSpeed`
  (params (percentileRecover :type "Float (double-precision)"))
  (set `self.movementSpeed` (/ (`self.movementSpeed`) percentileRecover)))

(fn `RecoverPercentileMaxHP`
  (params (maxRecovAmount :type "Float (double-precision)"))
  (set `self.maxHP` (/ (`self.maxHP`) maxRecovAmount)))

(fn `ReduceHPDirect`
  (params (reductionAmount :type "Float (double-precision)"))
  (set `self.HP` (`KismetMathLibrary.FClamp` (- (`self.HP`) reductionAmount) 0.0 (`self.maxHP`))))

(fn `ReduceSpellSlot`
  (params (reduceAmount :type "Float (double-precision)"))
  (set `self.SpellSlots` (`KismetMathLibrary.FClamp` (- reduceAmount (`self.SpellSlots`)) 0.0 (`self.maxSpellSlots`))))

(fn `ReduceStamina`
  (params (staminaReduction :type Integer :default 0))
  (returns (isExhausted :type Boolean))
  (set `self.curStamina` (`KismetMathLibrary.Clamp` (- (`self.curStamina`) staminaReduction) 0 999))
  (return (`self.CheckForExhaustion`)))

(fn `SetAllStats by Struct`
  (params (`Data to Load` :type "/Game/Scripts/Blueprints/System/Data/PlayerSaveData Structure"))
  (set `self.maxHP` `Data to Load_maxHP_26_DDAC747441D4BBB33BD2E3B29DCBAA0E`)
  (set `self.HP` `Data to Load_HP_27_AB26E7664D97C2E1BA628888C8AEF2D1`)
  (set `self.ATK` `Data to Load_ATK_28_5EE31C514A16EF4D628EF6993747988E`)
  (set `self.DEF` `Data to Load_DEF_29_7ED19C20413796B214F18580475E0078`)
  (set `self.Money` `Data to Load_Money_33_A3C316F24D56CAD1D6737596D31440C7`)
  (set `self.maxSpellSlots` `Data to Load_maxSpellSlots_42_AEEB566A4B4AF1987B72AAA5C6C6B3F0`)
  (set `self.SpellSlots` `Data to Load_SpellSlots_43_70BAEE0C43437C1ABDE88C8CD28C675B`)
  (set `self.LUK` `Data to Load_LUK_36_E68361EE40CA926816DBFFB8A2FEB053`)
  (set `self.critModifier` `Data to Load_critMod_37_67A2B49946C415244C174D8167B91B27`)
  (set `self.Name` `Data to Load_Name_38_2FE0CE1B485FE9E1FA17E7961C0033AA`)
  (set `self.curStamina` `Data to Load_Exhaust_41_6EDB461141AA277C94B91A88C5E1D766`)
  (set `self.movementSpeed` `Data to Load_movementSpeed_46_62B4086E4BD9F31BCBCC29A6AC41DE33`))

(fn `SetDEF`
  (params (DEFChange :type "Float (double-precision)") (isPercentile :type Boolean))
  (if isPercentile
    (set `self.DEF` (* (`self.DEF`) DEFChange))
    (else
      (set `self.DEF` (+ (`self.DEF`) DEFChange)))))

(fn `SetGoats`
  (params (goatsAdded :type Integer))
  (set `self.Goat` (+ goatsAdded (`self.Goat`))))

(fn `SetHP`
  (params (hpAdded :type "Float (double-precision)"))
  (set `self.HP` (`KismetMathLibrary.FClamp` (+ hpAdded (`self.HP`)) 0.0 (`self.maxHP`))))

(fn `SetMAXHP`
  (params (newMaxHP :type "Float (double-precision)"))
  (bind _output_get (set `self.maxHP` newMaxHP))
  (if (>= (`self.HP`) _output_get)
    (set `self.HP` _output_get)))

(fn `SetMAXHPAdhjusted`
  (params (MaxHPChange :type "Float (double-precision)") (isPercentile :type Boolean))
  (if isPercentile
    (set `self.maxHP` (* (`self.maxHP`) MaxHPChange))
    (else
      (set `self.maxHP` (+ (`self.maxHP`) MaxHPChange))))
  (set `self.HP` (`KismetMathLibrary.FClamp` (`self.HP`) 0.0 (`self.maxHP`))))

(fn `SetMoney`
  (params (moneyChange :type Integer))
  (bind _returnvalue (`KismetStringLibrary.Conv_IntToString` moneyChange))
  (set `self.Money` (+ (`self.Money`) moneyChange))
  (if (>= moneyChange 0)
    (bind _returnvalue_2 (`|CreateWidget` "/Game/Scripts/Blueprints/UI/MainHUD/MoneyChanged.MoneyChanged_C" null _returnvalue))
    (`UserWidget.AddToViewport` _returnvalue_2 0)
    (else
      (bind _returnvalue_3 (`|CreateWidget` "/Game/Scripts/Blueprints/UI/MainHUD/MoneyChanged.MoneyChanged_C" null _returnvalue true))
      (`UserWidget.AddToViewport` _returnvalue_3 0))))

(fn `SetMovementSpeed`
  (params (percentileChange :type "Float (double-precision)"))
  (set `self.movementSpeed` (* (`self.movementSpeed`) percentileChange)))

(fn `TakeDamage`
  (params (`Damage Taken` :type "Float (double-precision)") (wasCrit :type Boolean) (DamageType :type "/Game/Scripts/Blueprints/System/ElementType Enum" :default "NewEnumerator0") (TotalBonusDEF :type "Float (double-precision)") (`Lowest Damage` :type "Float (double-precision)"))
  (locals (ReceivedDamage :type "Float (double-precision)") (BonusDef :type "Float (double-precision)") (BonusRes :type "Float (double-precision)") (LowestDamageTaken :type "Float (double-precision)") (isCrit :type Boolean))
  (bind _returnvalue (- (* `Damage Taken` (`self.EvaluateElementalAffinity` DamageType)) TotalBonusDEF))
  (set `self.HP` (`self.ReduceHP` _returnvalue))
  (`self.DisplayDamage` _returnvalue wasCrit))

(fn `TakeDirectDamage`
  (params (DamageIn :type "Float (double-precision)")))