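; GetUtilities is a helper library giving shared access to the game instance, game mode, player character, controller, stats and UI.
; Getters cast the engine's objects to project classes, assuming player index 0, and the UI getter takes the first top-level PlayerUI widget.
; Direction helpers read the character's Sprite: the sign of its forward X gives left/right facing, and offsets scale by that X with Y and Z fixed at one.
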(fn `GetBasePlayerController`
  (returns (`AsBase Player Controller` :type "/Game/Scripts/Blueprints/Characters/Player/BasePlayerController Object Reference"))
  (bind _asbase_player_controller (cast `/Game/Scripts/Blueprints/Characters/Player/BasePlayerController` (`GameplayStatics.GetPlayerController` null)))
  (return _asbase_player_controller))

(fn `GetMyGameInstance`
  (returns (`AsMy Game Instance` :type "/Game/Scripts/Blueprints/MyGameInstance Object Reference"))
  (bind _asmy_game_instance (cast `/Game/Scripts/Blueprints/MyGameInstance` (`GameplayStatics.GetGameInstance` null)))
  (return _asmy_game_instance))

(fn `GetPlayerCharacter`
  (returns (`AsBase Character` :type "/Game/Scripts/Blueprints/Characters/Player/BaseCharacter Object Reference"))
  (bind _asbase_character (cast `/Game/Scripts/Blueprints/Characters/Player/BaseCharacter` (`GameplayStatics.GetPlayerCharacter` null)))
  (`/Engine/EditorBlueprintResources/StandardMacros.IsValid` _asbase_character
    (:`Is Valid`
      (return _asbase_character))))

(fn `GetPlayerForwardOffset`
  (params (offsetDistance :type "Vector Structure"))
  (returns (offsetPoint :type "Vector Structure"))
  (bind _asbase_character (`self.GetPlayerCharacter` null))
  (bind _returnvalue_x (`KismetMathLibrary.BreakVector` (`SceneComponent.GetForwardVector` (`PaperCharacter.Sprite` _asbase_character))))
  (return (+ (* offsetDistance (`KismetMathLibrary.MakeVector` _returnvalue_x 1.0 1.0)) (`Actor.K2_GetActorLocation` _asbase_character))))

(fn `GetPlayerForwardVector`
  (returns (playerForwardVector :type "Vector Structure"))
  (bind _returnvalue_x (`KismetMathLibrary.BreakVector` (`SceneComponent.GetForwardVector` (`PaperCharacter.Sprite` (`self.GetPlayerCharacter` null)))))
  (return (`KismetMathLibrary.MakeVector` _returnvalue_x 1.0 1.0)))

(fn `GetPlayerRotation`
  (returns (playerRotation :type "Rotator Structure"))
  (return (`SceneComponent.K2_GetComponentRotation` (`PaperCharacter.Sprite` (`self.GetPlayerCharacter` null)))))

(fn `GetPlayerStats`
  (returns (Stats :type "/Game/Scripts/Blueprints/System/Stats Object Reference"))
  (bind _asbase_character (cast `/Game/Scripts/Blueprints/Characters/Player/BaseCharacter` (`GameplayStatics.GetPlayerCharacter` null)))
  (return (`/Game/Scripts/Blueprints/Characters/Player/BaseCharacter.Stats` _asbase_character)))

(fn `GetPlayerUI`
  (returns (playerUI :type "/Game/Scripts/Blueprints/UI/MainHUD/PlayerUI Object Reference"))
  (bind _foundwidgets (`WidgetBlueprintLibrary.GetAllWidgetsOfClass` null "/Game/Scripts/Blueprints/UI/MainHUD/PlayerUI.PlayerUI_C"))
  (return (`|GetArrayItem` _foundwidgets)))

(fn `GetThisGameMode`
  (returns (`AsCapstone 2Rules` :type "/Game/Scripts/Blueprints/Capstone2Rules Object Reference"))
  (bind _ascapstone_2rules (cast `/Game/Scripts/Blueprints/Capstone2Rules` (`GameplayStatics.GetGameMode` null)))
  (return _ascapstone_2rules))

(fn `IsPlayerFacingRight`
  (returns (isRight :type Boolean))
  (`/Engine/EditorBlueprintResources/StandardMacros.CompareFloat` (.x (`self.GetPlayerForwardVector` null))
    (:`>`
      (return true))
    (:`<`
      (return false))))