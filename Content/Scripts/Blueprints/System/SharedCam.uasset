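; Shared orthographic camera actor that frames two local players and keeps them within a maximum separation.
; When players have spawned or NewPlayer fires, it blends both controllers' views to itself and caches the two actors tagged "Player".
; Each tick it moves to their midpoint and widens the ortho width with their distance.
; It then repositions both players symmetrically around that midpoint, clamping their separation to MaximumSize.
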(event `self.ReceiveBeginPlay`
  (bind _asmy_game_instance (cast `/Game/Scripts/Blueprints/MyGameInstance` (`GameplayStatics.GetGameInstance`)))
  (if (`/Game/Scripts/Blueprints/MyGameInstance.hasSpawned` _asmy_game_instance)
    (`PlayerController.SetViewTargetWithBlend` (`GameplayStatics.GetPlayerController` 0) self 2.0 "VTBlend_Linear" 0.0 false :!label _label)
    (`PlayerController.SetViewTargetWithBlend` (`GameplayStatics.GetPlayerController` 1) self 2.0 "VTBlend_Linear" 0.0 false)
    (bind _outactors (`GameplayStatics.GetAllActorsWithTag` "Player"))
    (set `self.C1` (`|GetArrayItem` _outactors))
    (set `self.C2` (`|GetArrayItem` _outactors 1))))

(event `New Player`
  (goto _label))

(event `self.ReceiveTick`
  (params (DeltaSeconds :type "Float (single-precision)"))
  (bind _returnvalue (`self.K2_GetActorLocation`))
  (bind _c1 (`self.C1`))
  (bind _distance (`self.Distance`))
  (bind _returnvalue_2 (/ (`KismetMathLibrary.ClampVectorSize` (`self.Distance`) 0.0 (`self.MaximumSize`)) 2.0))
  (if (`KismetSystemLibrary.IsValid` _c1)
    (set `self.Distance` (- (`self.K2_GetActorLocation` _c1) (`self.K2_GetActorLocation` (`self.C2`))))
    (`|ExecutionSequence`
      (:`then_0`
        (`self.K2_SetActorLocation` (+ (`self.K2_GetActorLocation` (`self.C2`)) (/ _distance 2.0)))
        (`CameraComponent.SetOrthoWidth` (`self.Camera`) (+ 1660.0 (`KismetMathLibrary.VSize` _distance))))
      (:`then_1`
        (`self.K2_SetActorLocation` (`self.C1`) (+ _returnvalue _returnvalue_2) false false)
        (`self.K2_SetActorLocation` (`self.C2`) (- _returnvalue _returnvalue_2) false false)))))

(fn `UserConstructionScript`)