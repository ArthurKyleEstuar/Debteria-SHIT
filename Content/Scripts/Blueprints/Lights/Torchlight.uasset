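; Torchlight is a light Blueprint that applies a configurable color to its point light and can make it flicker like a torch.
; On BeginPlay, a flickering light randomly plays one of three timelines, so separate instances can vary, while a steady light just uses IntensityFactor as its intensity.
; SetLight converts each timeline value into intensity using variance, base intensity and an overall factor.
; RandomizeTimeline and the construction script are empty.
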(event `self.ReceiveBeginPlay`
  (`LightComponent.SetLightColor` (`self.PointLightComponent`) (`self.LightColor`) true)
  (if (`self.isFlickering`)
    (switch `int` (`KismetMathLibrary.RandomIntegerInRange` 0 2)
      (:`0`
        (bind (_direction _lightintensity) (`Timeline|Flicker`)
          (:`Update`
            (`self.SetLight` _lightintensity))))
      (:`1`
        (bind (_direction_2 _lightintensity_2) (`Timeline|Flicker2`)
          (:`Update`
            (`self.SetLight` _lightintensity_2))))
      (:`2`
        (bind (_direction_3 _lightintensity_3) (`Timeline|Flicker3`)
          (:`Update`
            (`self.SetLight` _lightintensity_3)))))
    (else
      (`LightComponent.SetIntensity` (`self.PointLightComponent`) (`self.IntensityFactor`)))))

(fn `RandomizeTimeline`)

(fn `SetLight`
  (params (A :type "Float (double-precision)"))
  (`LightComponent.SetIntensity` (`self.PointLightComponent`) (* (+ (* A (`self.IntensityVariance`)) (`self.baseLightIntensity`)) (`self.IntensityFactor`))))

(fn `UserConstructionScript`)