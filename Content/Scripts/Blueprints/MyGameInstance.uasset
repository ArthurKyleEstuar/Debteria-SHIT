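; Game instance that carries campaign state across levels: debt, the day countdown to a final judgement, saved data and tutorial flags.
; One active quest struct is rebuilt as kills, interactions, pickups or wave clears advance it, pinging the player UI when complete.
; Starting a quest randomizes the spawner element; completing or failing drains stamina and archives it.
; Day changes run through widget callbacks that reset stats and reload the Tavern.
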(event `SetPreviousInputType`
  (params (isKeyboard :type Boolean))
  (set `self.wasKeyboard` isKeyboard))

(event `ReduceDebt`
  (params (amountPaid :type Integer))
  ;[1 1 1] Bring us the girl and wipe away the debt
  (set `self.currentDebt` (`KismetMathLibrary.Clamp` (- (`self.currentDebt`) amountPaid) 0 99999999)))

(event `AdvanceDay`
  (bind _daysremaining (`self.daysRemaining`))
  ;[1 1 1] Next day
  (if (`self.finalDay`)
    (`/Game/Scripts/Blueprints/Characters/Player/BaseCharacter.Save Data` (`/Game/Scripts/Blueprints/System/GetUtilities.GetPlayerCharacter`))
    (bind _returnvalue (`|CreateWidget` "/Game/Scripts/Blueprints/UI/IntroOutro/Judge.Judge_C"))
    (`UserWidget.AddToViewport` _returnvalue 0)
    (elif (> _daysremaining 1)
      (bind _returnvalue_2 (`|CreateWidget` "/Game/Scripts/Blueprints/UI/SpecialEffectsUI/NextDayUI.NextDayUI_C" null _daysremaining))
      (`UserWidget.AddToViewport` _returnvalue_2 2)
      (add `/Game/Scripts/Blueprints/UI/SpecialEffectsUI/NextDayUI.DayTransitioned` _returnvalue_2 (delegate `NextDayAdvance`))
      (else
        (bind _returnvalue_3 (`|CreateWidget` "/Game/Scripts/Blueprints/UI/SpecialEffectsUI/FInalDayNotif.FInalDayNotif_C" null _daysremaining))
        (`UserWidget.AddToViewport` _returnvalue_3 0)
        (add `/Game/Scripts/Blueprints/UI/SpecialEffectsUI/FInalDayNotif.DayFinalMode` _returnvalue_3 (delegate `FinalDayAdvance`))))))

(event `NextDayAdvance`
  ;[1 1 1] Next day
  (`self.ResetDayStats`)
  (`GameplayStatics.OpenLevel` "Tavern"))

(event `FinalDayAdvance`
  ;[1 1 1] Next day
  (`self.ResetDayStats`)
  (set `self.finalDay` true)
  (`GameplayStatics.OpenLevel` "Tavern"))

(event `RestartProgress`
  (set `self.currentDebt` (`self.initialDebt`))
  (set `self.daysRemaining` 5)
  (set `self.QuestTracker` (struct))
  (set `self.QuestOngoing` false)
  (set `self.MageData` (struct))
  (set `self.SavedInventory` (`|MakeArray` null :!type "/Game/Scripts/Blueprints/Characters/Player/Inventory/Items/Item_Object Class Reference"))
  (set `self.robeSavedData` (struct))
  (set `self.itemSavedData` (`|MakeArray` (struct) :!type "/Game/Scripts/Blueprints/Characters/Player/Inventory/ItemData Structure"))
  (set `self.SavedRunes` (`|MakeArray` (struct) :!type "/Game/Scripts/Blueprints/Characters/Player/Spells/Rune/RuneInventoryData Structure"))
  (set `self.SavedRobes` (`|MakeArray` (struct) :!type "/Game/Scripts/Blueprints/Characters/Player/Equipment/Robes/RobeData Structure")))

(event `PlayTutorialPrompt`
  (params (tutorialName :type Name))
  (bind (_tutorialdisplay _tutorialprompted) (break `/Game/Scripts/Blueprints/TutorialData` (`self.HasTutorialAvailable` tutorialName (`self.tutorials`))))
  (if (not _tutorialprompted)
    (`BlueprintMapLibrary.Map_Add` (`self.tutorials`) tutorialName (make `/Game/Scripts/Blueprints/TutorialData` _tutorialdisplay true))
    (bind _returnvalue (`|CreateWidget` "/Game/Scripts/Blueprints/UI/HelperUI.HelperUI_C" null _tutorialdisplay))
    (`UserWidget.AddToViewport` _returnvalue 2)
    (add `/Game/Scripts/Blueprints/UI/HelperUI.EndHelp` _returnvalue (delegate `HelpEnd`))
    (else
      (`self.HelpEnd`))))

(event `HelpEnd`
  (`self.HelpEnded`))

(event `Quest Interacted`
  (bind (_questtracker_questname _questtracker_questdescription _questtracker_questtype _questtracker_questtarget _questtracker_questitemtarget _questtracker_questinteracttarget _questtracker_questprogress _questtracker_questminimumprogress _questtracker_questsilverprogress _questtracker_questgoldprogress _questtracker_questcompleted _questtracker_exhaustinflict _questtracker_moneyreward _questtracker_questprogressionmod _questtracker_questlocation _questtracker_questdayunlock _questtracker_questprerequisite _questtracker_questportrait) (break `/Game/Scripts/Blueprints/System/Quests/QuestData` (`self.QuestTracker`)))
  ;[1 1 1] Add Quest Item
  (bind _result (`/Engine/EditorBlueprintResources/StandardMacros.IncrementInt` _questtracker_questprogress :!label _label)
    (:`  `
      (bind _returnvalue (>= _result _questtracker_questminimumprogress))
      (set `self.QuestTracker` (make `/Game/Scripts/Blueprints/System/Quests/QuestData` _questtracker_questname _questtracker_questdescription _questtracker_questtype _questtracker_questtarget _questtracker_questitemtarget _questtracker_questinteracttarget _questtracker_questprogress _questtracker_questminimumprogress _questtracker_questsilverprogress _questtracker_questgoldprogress _returnvalue _questtracker_exhaustinflict _questtracker_moneyreward _questtracker_questprogressionmod _questtracker_questlocation _questtracker_questdayunlock _questtracker_questprerequisite _questtracker_questportrait))
      (if _returnvalue
        (`self.Ping`)))))

(event `Quest Item Picked up`
  ;[1 1 1] Add Quest Item
  (goto _label))

(event `Check WaveQuest Finished`
  ;[1 1 1] Wave Clear
  (if (`.QuestCompleted_20_B231AFB445E11E8341A60FA4E7C3BBAE` (break `/Game/Scripts/Blueprints/System/Quests/QuestData` (`self.QuestTracker`)))
    (bind _returnvalue (`|CreateWidget` "/Game/Scripts/Blueprints/UI/QuestsUI/WaveSurvived.WaveSurvived_C"))
    (`UserWidget.AddToViewport` _returnvalue 0)))

(event `EnemyKilled_Event`
  (params (killedEnemyType :type "/Game/Scripts/Blueprints/Characters/Enemies/BaseAI Class Reference"))
  (bind (_questtracker_questname _questtracker_questdescription _questtracker_questtype _questtracker_questtarget _questtracker_questitemtarget _questtracker_questinteracttarget _questtracker_questprogress _questtracker_questminimumprogress) (break `/Game/Scripts/Blueprints/System/Quests/QuestData` (`self.QuestTracker`)))
  (bind (_questtracker_questname_2 _questtracker_questdescription_2 _questtracker_questtype_2 _questtracker_questtarget_2 _questtracker_questitemtarget_2 _questtracker_questinteracttarget_2 _questtracker_questprogress_2 _questtracker_questminimumprogress_2 _questtracker_questsilverprogress _questtracker_questgoldprogress _questtracker_questcompleted _questtracker_exhaustinflict _questtracker_moneyreward _questtracker_questprogressionmod _questtracker_questlocation _questtracker_questdayunlock _questtracker_questprerequisite _questtracker_questportrait) (break `/Game/Scripts/Blueprints/System/Quests/QuestData` (`self.QuestTracker`)))
  ;[1 1 1] Update Kill Quest
  (if (and (== killedEnemyType _questtracker_questtarget) (or (`|EnumEquality` _questtracker_questtype "NewEnumerator0") (`|EnumEquality` _questtracker_questtype "NewEnumerator5")))
    (bind _result (`/Engine/EditorBlueprintResources/StandardMacros.IncrementInt` _questtracker_questprogress)
      (:`  `
        (bind _returnvalue (>= _result _questtracker_questminimumprogress))
        (set `self.QuestTracker` (make `/Game/Scripts/Blueprints/System/Quests/QuestData` _questtracker_questname_2 _questtracker_questdescription_2 _questtracker_questtype_2 _questtracker_questtarget_2 _questtracker_questitemtarget_2 _questtracker_questinteracttarget_2 _questtracker_questprogress_2 _questtracker_questminimumprogress_2 _questtracker_questsilverprogress _questtracker_questgoldprogress _returnvalue _questtracker_exhaustinflict _questtracker_moneyreward _questtracker_questprogressionmod _questtracker_questlocation _questtracker_questdayunlock _questtracker_questprerequisite _questtracker_questportrait))
        (if _returnvalue
          (`self.Ping`))))))

(event `SetQuest`
  (params (QuestToTrack :type "/Game/Scripts/Blueprints/System/Quests/QuestData Structure"))
  ;[1 1 1] Activate Quest
  (set `self.QuestTracker` QuestToTrack)
  (set `self.QuestOngoing` true)
  (`self.RandomizeEnemyElement`)
  (bind _returnvalue (`|CreateWidget` "/Game/Scripts/Blueprints/UI/QuestsUI/QuestAddUpdateNotification.QuestAddUpdateNotification_C"))
  (`UserWidget.AddToViewport` _returnvalue 0))

(event `Force Complete`
  (bind (_questtracker_questname _questtracker_questdescription _questtracker_questtype _questtracker_questtarget _questtracker_questitemtarget _questtracker_questinteracttarget _questtracker_questprogress _questtracker_questminimumprogress _questtracker_questsilverprogress _questtracker_questgoldprogress _questtracker_questcompleted _questtracker_exhaustinflict) (break `/Game/Scripts/Blueprints/System/Quests/QuestData` (`self.QuestTracker`)))
  ;[1 1 1] End Quest
  (set `self.QuestOngoing` false :!label _label_2)
  (set `self.questItemAccumulated` 0)
  (`/Game/Scripts/Blueprints/System/Stats.ReduceStamina` (`/Game/Scripts/Blueprints/Characters/Player/BaseCharacter.Stats` (`/Game/Scripts/Blueprints/System/GetUtilities.GetPlayerCharacter`)) _questtracker_exhaustinflict)
  (bind _returnvalue (`self.ClearQuestAndNotify`))
  (add `/Game/Scripts/Blueprints/UI/QuestsUI/QuestCompleted.UIClosed` _returnvalue (delegate `RollRandomEvent`)))

(event `exhaust`
  ;[1 1 1] End Quest
  ;;[1 1 1] Exhaust After Quest
  (if (`/Game/Scripts/Blueprints/System/Stats.CheckForExhaustion` (`/Game/Scripts/Blueprints/Characters/Player/BaseCharacter.Stats` (`/Game/Scripts/Blueprints/System/GetUtilities.GetPlayerCharacter`)))
    (bind _returnvalue (`|CreateWidget` "/Game/Scripts/Blueprints/UI/MenusUI/ExertUI.ExertUI_C"))
    (`UserWidget.AddToViewport` _returnvalue 2)))

(event `CompleteQuest`
  (bind (_questtracker_questname _questtracker_questdescription _questtracker_questtype _questtracker_questtarget _questtracker_questitemtarget _questtracker_questinteracttarget _questtracker_questprogress _questtracker_questminimumprogress _questtracker_questsilverprogress _questtracker_questgoldprogress _questtracker_questcompleted _questtracker_exhaustinflict) (break `/Game/Scripts/Blueprints/System/Quests/QuestData` (`self.QuestTracker`)))
  ;[1 1 1] End Quest
  (if _questtracker_questcompleted
    (goto _label_2)))

(event `RollRandomEvent`
  ;[1 1 1] End Quest
  (`/Game/Scripts/Blueprints/Capstone2Rules.Roll Event System` (`/Game/Scripts/Blueprints/System/GetUtilities.GetThisGameMode`)))

(event `Fail Quest`
  (bind _asbase_character (`/Game/Scripts/Blueprints/System/GetUtilities.GetPlayerCharacter`))
  ;[1 1 1] QuestFailed
  (`GameplayStatics.SetGamePaused` true)
  (set `self.QuestOngoing` false)
  (`self.ClearAndArchiveQuest`)
  (bind _isexhausted (`/Game/Scripts/Blueprints/System/Stats.ReduceStamina` (`/Game/Scripts/Blueprints/Characters/Player/BaseCharacter.Stats` _asbase_character) 1))
  (`self.SavePlayer`)
  (if _isexhausted
    (`/Game/Scripts/Blueprints/Characters/Player/BaseCharacter.Revive` _asbase_character)
    (`/Game/Scripts/Blueprints/Characters/Player/BaseCharacter.BusyInteracting` _asbase_character)
    (bind _returnvalue (`|CreateWidget` "/Game/Scripts/Blueprints/UI/SpecialEffectsUI/ExhaustUI.ExhaustUI_C"))
    (`UserWidget.AddToViewport` _returnvalue 0)
    (add `/Game/Scripts/Blueprints/UI/SpecialEffectsUI/ExhaustUI.Exhausted` _returnvalue (delegate `ExhaustedFinished`))
    (`KismetSystemLibrary.Delay` 1.0)
    (`GameplayStatics.SetGamePaused` true)
    (else
      (`/Game/Scripts/Blueprints/Characters/Player/BaseCharacter.Revive` _asbase_character)
      (`GameplayStatics.OpenLevel` "Tavern"))))

(event `ExhaustedFinished`
  ;[1 1 1] QuestFailed
  (`self.ClearAndArchiveQuest`)
  (`self.AdvanceDay`))

(event `FailQuestNoRevive`
  ;[1 1 1] QuestFailed
  (set `self.QuestOngoing` false)
  (`self.ClearAndArchiveQuest`)
  (bind _isexhausted (`/Game/Scripts/Blueprints/System/Stats.ReduceStamina` (`/Game/Scripts/Blueprints/Characters/Player/BaseCharacter.Stats` (`/Game/Scripts/Blueprints/System/GetUtilities.GetPlayerCharacter`)) 1))
  (if (not _isexhausted)
    (`GameplayStatics.OpenLevel` "Tavern")))

(event `Clear Quest`
  ;[1 1 1] Submitted Quest
  (set `self.QuestOngoing` false)
  (`self.ClearAndArchiveQuest`)
  (`self.QuestEnded`))

(fn `AddStoryQuestCompleted`
  (params (storyQuestCompleted :type String))
  (for _array_element (`self.completedStoryQuests`)
    (if (`KismetStringLibrary.EqualEqual_StrStr` storyQuestCompleted _array_element)
      (return)))
  (`KismetArrayLibrary.Array_Add` (`self.completedStoryQuests`) storyQuestCompleted))

(fn `CheckWavesCleared`
  (returns (isFinished :type Boolean))
  (bind (_questtracker_questname _questtracker_questdescription _questtracker_questtype _questtracker_questtarget _questtracker_questitemtarget _questtracker_questinteracttarget _questtracker_questprogress _questtracker_questminimumprogress _questtracker_questsilverprogress _questtracker_questgoldprogress _questtracker_questcompleted _questtracker_exhaustinflict _questtracker_moneyreward _questtracker_questprogressionmod _questtracker_questlocation _questtracker_questdayunlock) (break `/Game/Scripts/Blueprints/System/Quests/QuestData` (`self.QuestTracker`)))
  (bind _result (`/Engine/EditorBlueprintResources/StandardMacros.IncrementInt` _questtracker_questprogress)
    (:`  `
      (bind _returnvalue (>= _result _questtracker_questminimumprogress))
      (set `self.QuestTracker` (make `/Game/Scripts/Blueprints/System/Quests/QuestData` _questtracker_questname _questtracker_questdescription _questtracker_questtype _questtracker_questtarget null null _questtracker_questprogress _questtracker_questminimumprogress _questtracker_questsilverprogress _questtracker_questgoldprogress _returnvalue _questtracker_exhaustinflict _questtracker_moneyreward _questtracker_questprogressionmod _questtracker_questlocation _questtracker_questdayunlock))
      (`self.Check WaveQuest Finished`)
      (if _returnvalue
        (`self.Ping`)
        (`self.WavesCompleted`)
        (return true)
        (else
          (return false))))))

(fn `ClearAndArchiveQuest`
  (`KismetArrayLibrary.Array_Add` (`self.PastCompletedQuests`) (`self.QuestTracker`))
  (set `self.QuestTracker` (make `/Game/Scripts/Blueprints/System/Quests/QuestData` "")))

(fn `ClearQuestAndNotify`
  (returns (ReturnValue :type "/Game/Scripts/Blueprints/UI/QuestsUI/QuestCompleted Object Reference"))
  (bind _returnvalue (`|CreateWidget` "/Game/Scripts/Blueprints/UI/QuestsUI/QuestCompleted.QuestCompleted_C" null (`self.QuestTracker`)))
  (`UserWidget.AddToViewport` _returnvalue 0)
  (`self.ClearAndArchiveQuest`)
  (`self.QuestEnded`)
  (return _returnvalue))

(fn `GetCurrentDay`
  (returns (curDay :type Integer))
  (return (`KismetMathLibrary.Abs_Int` (- (`self.daysRemaining`) 5))))

(fn `HasTutorialAvailable`
  (params (tutorialName :type "Name (by ref)") (tutoralMap :type "Map of Name to /Game/Scripts/Blueprints/TutorialData Structure (by ref)"))
  (returns (tutorialData :type "/Game/Scripts/Blueprints/TutorialData Structure"))
  (return (`BlueprintMapLibrary.Map_Find` tutoralMap tutorialName)))

(fn `IsEndOfGame`
  (returns (isTheEnd :type Boolean))
  (return (<= (`self.daysRemaining`) -1)))

(fn `Ping`
  (bind _foundwidgets (`WidgetBlueprintLibrary.GetAllWidgetsOfClass` "/Game/Scripts/Blueprints/UI/MainHUD/PlayerUI.PlayerUI_C"))
  (`/Game/Scripts/Blueprints/UI/MainHUD/PlayerUI.Completed Ping` (`|GetArrayItem` _foundwidgets)))

(fn `RandomizeEnemyElement`
  (locals (elements :type "Array of /Game/Scripts/Blueprints/System/ElementType Enum"))
  (bind _elements (`local.elements`))
  (for _ (range 4)
    (`KismetArrayLibrary.Array_Shuffle` _elements))
  (set `self.spawnerElement` (`|GetArrayItem` _elements)))

(fn `ResetDayStats`
  (bind _asbase_character (`/Game/Scripts/Blueprints/System/GetUtilities.GetPlayerCharacter`))
  (set `/Game/Scripts/Blueprints/System/Stats.curStamina` 2 (`/Game/Scripts/Blueprints/Characters/Player/BaseCharacter.Stats` _asbase_character))
  (`/Game/Scripts/Blueprints/Characters/Player/BaseCharacter.Save Data` _asbase_character)
  (`/Engine/EditorBlueprintResources/StandardMacros.DecrementInt` (`self.daysRemaining`)
    (:`  `
      (`self.IsEndOfGame`))))

(fn `ResetTempValues`
  (set `self.tempTax` 0.0)
  (set `self.tempLivingExpense` 0.0))

(fn `SavePlayer`
  (`/Game/Scripts/Blueprints/Characters/Player/BaseCharacter.Save Data` (`/Game/Scripts/Blueprints/System/GetUtilities.GetPlayerCharacter`)))

(fn `SetHelpPrompted`
  (params (isPrompted :type Boolean))
  (bind _tutorials (`self.tutorials`))
  (bind _values (`BlueprintMapLibrary.Map_Values` _tutorials))
  (for (_array_element _array_index) _values
    (bind _keys (`BlueprintMapLibrary.Map_Keys` _tutorials))
    (`BlueprintMapLibrary.Map_Add` _tutorials (`|GetArrayItem` _keys _array_index) (make `/Game/Scripts/Blueprints/TutorialData` (`.TutorialDisplay_3_A8C168FD453172C004ADED8ADB951E12` (break `/Game/Scripts/Blueprints/TutorialData` _array_element)) isPrompted))))