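; Game mode for the Capstone2 project that handles spawning the player's Mage and relays rolls to a random event system.
; On BeginPlay, if the game instance's HasSpawned flag is set, it makes Mage the default pawn, spawns one at the first PlayerStart and possesses it.
; DebugSpawn sets that flag and runs the same spawn path.
; RollSystem triggers RollForEvent, and SetSpawnWaveEnemy stores the wave's enemy in WaveAI.
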(event `Roll Event System`
  (`/Game/Scripts/Blueprints/System/RandomEvents/RandomEventSystem.Roll for Event` (`self.RandomEventSystem`)))

(event `self.ReceiveBeginPlay`
  (if (`/Game/Scripts/Blueprints/MyGameInstance.hasSpawned` (`/Game/Scripts/Blueprints/System/GetUtilities.GetMyGameInstance`))
    (set `self.DefaultPawnClass` "/Game/Scripts/Blueprints/Characters/Player/Mage.Mage_C" :!label _label)
    (`self.SpawnMage` (`GameplayStatics.GetPlayerController` 0))))

(event `Debug Spawn`
  (set `/Game/Scripts/Blueprints/MyGameInstance.hasSpawned` true (`/Game/Scripts/Blueprints/System/GetUtilities.GetMyGameInstance`))
  (goto _label))

(fn `SetSpawnWaveEnemy`
  (params (enemyWave :type "/Game/Scripts/Blueprints/Characters/Enemies/BaseAI Class Reference"))
  (set `self.waveAI` enemyWave))

(fn `SpawnMage`
  (params (Controller :type "PlayerController Object Reference"))
  (locals (NewLocalVar_0 :type "Transform Structure"))
  (bind _outactors (`GameplayStatics.GetAllActorsOfClass` "/Script/Engine.PlayerStart"))
  (bind (_returnvalue_x _returnvalue_y _returnvalue_z) (`KismetMathLibrary.BreakVector` (`self.K2_GetActorLocation` (`|GetArrayItem` _outactors))))
  (bind _returnvalue (`|SpawnActorFromClass` :`Class` "/Game/Scripts/Blueprints/Characters/Player/Mage.Mage_C" :`SpawnTransform` (`KismetMathLibrary.MakeTransform` (`KismetMathLibrary.MakeVector` _returnvalue_x _returnvalue_y _returnvalue_z)) :`CollisionHandlingOverride` "Undefined" :`TransformScaleMethod` "OverrideRootScale" :`Instigator` null))
  (`Controller.Possess` Controller _returnvalue))

(fn `UserConstructionScript`)