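; Dropped money pickup that passes its MoneyAmount to SetMoney on the player character's Stats, then destroys itself.
; A short delay after BeginPlay arms the pickup, then immediately collects it if any BaseCharacter already overlaps the Box.
; Later Box overlaps trigger the same collection only for components tagged PlayerHit once armed.
; The money always goes to the player character, whichever BaseCharacter was found in the initial check.
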(event `self.ReceiveBeginPlay`
  (`KismetSystemLibrary.Delay` 0.3)
  (set `self.canPickUp` true)
  (`/Engine/EditorBlueprintResources/StandardMacros.IsValid` (`|GetArrayItem` (`PrimitiveComponent.GetOverlappingActors` (`self.Box`) "/Game/Scripts/Blueprints/Characters/Player/BaseCharacter.BaseCharacter_C"))
    (:`Is Valid`
      (`/Game/Scripts/Blueprints/System/Stats.SetMoney` (`/Game/Scripts/Blueprints/Characters/Player/BaseCharacter.Stats` (`/Game/Scripts/Blueprints/System/GetUtilities.GetPlayerCharacter`)) (`self.moneyAmount`) :!label _label)
      (`self.K2_DestroyActor`))))

(event `self.Box.OnComponentBeginOverlap`
  (params (OverlappedComponent :type "PrimitiveComponent Object Reference") (OtherActor :type "Actor Object Reference") (OtherComp :type "PrimitiveComponent Object Reference") (OtherBodyIndex :type Integer) (bFromSweep :type Boolean) (SweepResult :type "HitResult Structure (by ref)"))
  (if (and (`ActorComponent.ComponentHasTag` OtherComp "PlayerHit") (`self.canPickUp`))
    (goto _label)))

(fn `UserConstructionScript`)